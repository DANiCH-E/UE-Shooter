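; Game mode that runs a kill-all-enemies mission, from start screen to win screen and level load.
; On BeginPlay it shows the mission start widget, counts every BP_AICharacter and binds to each one's death event.
; Each death decrements the counter; at zero, a DoOnce shows the win widget, unbinds the death events and opens BattleCity after a short delay, issued inside the unbind loop.
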(event Custom|OnKillingEnemy
  (bind _result (Math|Integer|DecrementInt (Variables|Default|GetNumberOfEnemies))
    (:%20%20
      (if (<= _result 0)
        (Utilities|FlowControl|DoOnce false
          (:Completed
            (bind _returnvalue (UserInterface|CreateWidget "/Game/Core/UI/WBP_Win.WBP_Win_C"))
            (UserInterface|Viewport|AddtoViewport _returnvalue 0)
            (bind _outactors (Actor|GetAllActorsOfClass "/Game/Core/Blueprints/Character/AICharacter/BP_AICharacter.BP_AICharacter_C"))
            (for _array_element _outactors
              (EventDispatchers|UnbindEventfromOnDeath _array_element (delegate Custom|OnKillingEnemy))
              (Utilities|FlowControl|Delay 3.0)
              (Game|OpenLevel(byName) "BattleCity"))))))))

(event EventBeginPlay
  (bind _returnvalue (UserInterface|CreateWidget "/Game/Core/UI/WBP_MissionStart.WBP_MissionStart_C"))
  (UserInterface|Viewport|AddtoViewport _returnvalue 0)
  (bind _outactors (Actor|GetAllActorsOfClass "/Game/Core/Blueprints/Character/AICharacter/BP_AICharacter.BP_AICharacter_C"))
  (Variables|Default|SetNumberOfEnemies (Utilities|Array|Length _outactors))
  (for _array_element _outactors
    (EventDispatchers|BindEventtoOnDeath _array_element (delegate Custom|OnKillingEnemy))))

(fn ConstructionScript)