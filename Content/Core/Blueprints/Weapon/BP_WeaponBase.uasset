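; Base weapon Blueprint that a character picks up through interaction, attaches to its right hand, drops as a physics object, fires and instantly reloads.
; Firing is single-shot or timer-looped automatic, updating the character's weapon info as ammo changes.
; Each shot runs a cone-spread hitscan trace, from the camera for the player or from the weapon toward a Blackboard target for other characters, applying damage and effects on hit.
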(event Custom|Equip
  (params (Character :type BP%20Base%20Character%20Object%20Reference))
  (bind _skeletalmesh (Variables|Default|GetSkeletalMesh))
  ;[1 1 1] Equip Weapon
  (bind _output_get (Variables|Default|SetCharacter Character))
  (Utilities|IsValid (Variables|/Game/Core/Blueprints/Character/BP_BaseCharacter.BP_BaseCharacter_C|GetActiveWeapon _output_get)
    (:Is%20Valid
      (CallFunction|Drop (Variables|/Game/Core/Blueprints/Character/BP_BaseCharacter.BP_BaseCharacter_C|GetActiveWeapon _output_get))
      (Utilities|FlowControl|Delay 0.2))
    (:Is%20Not%20Valid
      _))
  (Physics|SetSimulatePhysics _skeletalmesh false)
  (Collision|SetCollisionEnabled _skeletalmesh "NoCollision")
  (Variables|/Game/Core/Blueprints/Character/BP_BaseCharacter.BP_BaseCharacter_C|SetActiveWeapon (Variables|Default|GetCharacter) self)
  (Transformation|AttachComponentToComponent (Variables|/Game/Core/Blueprints/Character/BP_BaseCharacter.BP_BaseCharacter_C|GetRightHandScene (Variables|Default|GetCharacter)) "None" "SnapToTarget" "SnapToTarget" "KeepWorld" true)
  (Default|UpdateWeaponInfo (Variables|Default|GetCharacter)))

(event Custom|Reload
  (if (< (Variables|Default|GetCurrentAmmo) (Variables|Default|GetMaxAmmo))
    (Variables|Default|SetCurrentAmmo (Variables|Default|GetMaxAmmo))
    (Default|UpdateWeaponInfo (Variables|Default|GetCharacter))))

(event Custom|Drop
  (bind _skeletalmesh (Variables|Default|GetSkeletalMesh))
  ;[1 1 1] Drop Weapon
  (CallFunction|StopFiring)
  (Variables|/Game/Core/Blueprints/Character/BP_BaseCharacter.BP_BaseCharacter_C|SetActiveWeapon (Variables|Default|GetCharacter) 0)
  (Transformation|DetachFromActor "KeepWorld" "KeepWorld" "KeepWorld")
  (Collision|SetCollisionEnabled _skeletalmesh "QueryAndPhysics")
  (Physics|SetSimulatePhysics _skeletalmesh true)
  (Default|UpdateWeaponInfo (Variables|Default|GetCharacter)))

(event Custom|StartFiring
  (switch Utilities|FlowControl|Switch|SwitchonE_WeaponFiringType (Variables|Default|GetFiringType)
    (:NewEnumerator0
      (if (Utilities|Time|IsValidTimerHandle (Variables|Default|GetFiringTimer))
        (Utilities|Time|UnpauseTimerbyHandle)
        (else
          (bind _returnvalue (Utilities|Time|SetTimerbyEvent (EventDispatchers|CreateEvent :!event Custom|SingleFire) (Variables|Default|GetAutoFireDelay) true))
          (Variables|Default|SetFiringTimer _returnvalue))))
    (:NewEnumerator1
      (CallFunction|SingleFire))))

(event Custom|SingleFire
  (bind _returnvalue (Game|GetPlayerCameraManager 0))
  (bind _scene (Variables|Default|GetScene))
  (bind _returnvalue_2 (Transformation|GetActorLocation _returnvalue))
  (bind _returnvalue_3 (Transformation|GetWorldLocation _scene))
  (if (> (Variables|Default|GetCurrentAmmo) 0)
    (Variables|Default|SetCurrentAmmo (- (Variables|Default|GetCurrentAmmo) 1))
    (Default|UpdateWeaponInfo (Variables|Default|GetCharacter))
    (Audio|PlaySoundatLocation (Variables|Default|GetSingleFireSound) (Transformation|GetWorldLocation (Variables|Default|GetScene)) "0, 0, 0" 1.0 1.0 0.0 "/Game/MilitaryWeapDark/Sound/Attenuation/WeaponShot_att.WeaponShot_att" 0 0 0)
    (Effects|SpawnEmitterAttached "/Game/MilitaryWeapDark/FX/P_AssaultRifle_MuzzleFlash.P_AssaultRifle_MuzzleFlash" (Variables|Default|GetScene) "None" "0, 0, 0" "0, 0, 0" "1.000000,1.000000,1.000000" "SnapToTarget")
    (if (== (Utilities|GetClass (Variables|Default|GetCharacter)) "/Game/Core/Blueprints/Character/BP_PlayerCharacter.BP_PlayerCharacter_C")
      (bind (_outhit _returnvalue_4) (Collision|LineTraceByChannel _returnvalue_2 (+ _returnvalue_2 (* (Math|Random|RandomUnitVectorinConeinDegrees (Math|Vector|GetForwardVector (Pawn|GetControlRotation (Game|GetPlayerController 0) :!class /Script/Engine.Controller)) (Variables|Default|GetCone%20Half%20Angle%20in%20Degrees)) (Variables|Default|GetTraceDistance))) "TraceTypeQuery1" false 0 "None"))
      (if _returnvalue_4
        (Variables|Default|SetImpact%20Point (.ImpactPoint (Collision|BreakHitResult _outhit)))
        (Variables|Default|SetHit%20Actor (.HitActor (Collision|BreakHitResult _outhit)))
        (Effects|SpawnEmitteratLocation "/Game/MilitaryWeapDark/FX/P_Impact_Metal_Medium_01.P_Impact_Metal_Medium_01" (Variables|Default|GetImpact%20Point) :!label _label)
        (Game|Damage|ApplyDamage (Variables|Default|GetHit%20Actor) (Variables|Default|GetBase%20Damage) 0 (Variables|Default|GetCharacter))
        (Audio|PlaySoundatLocation (Variables|Default|GetHitSound) (Variables|Default|GetImpact%20Point) "0, 0, 0" 1.0 1.0 0.0 "/Game/MilitaryWeapDark/Sound/Attenuation/WeaponShot_att.WeaponShot_att" 0 0 0))
      (else
        (bind _asactor (Utilities|Casting|CastToActor (AI|Components|Blackboard|GetValueasObject (AI|GetBlackboard (Variables|Default|GetCharacter)) (Variables|Default|GetKey%20Name))))
        (bind (_outhit_2 _returnvalue_5) (Collision|LineTraceByChannel _returnvalue_3 (+ _returnvalue_3 (* (Math|Random|RandomUnitVectorinConeinDegrees (Math|Vector|GetUnitDirection(Vector) _returnvalue_3 (Transformation|GetActorLocation _asactor)) (Variables|Default|GetCone%20Half%20Angle%20in%20Degrees)) (Variables|Default|GetTraceDistance))) "TraceTypeQuery1" false 0 "ForDuration"))
        (if _returnvalue_5
          (Variables|Default|SetImpact%20Point (.ImpactPoint (Collision|BreakHitResult _outhit_2)))
          (Variables|Default|SetHit%20Actor (.HitActor (Collision|BreakHitResult _outhit_2)))
          (goto _label))))))

(event Custom|StopFiring
  (bind _firingtimer (Variables|Default|GetFiringTimer))
  (switch Utilities|FlowControl|Switch|SwitchonE_WeaponFiringType (Variables|Default|GetFiringType)
    (:NewEnumerator0
      (if (Utilities|Time|IsValidTimerHandle _firingtimer)
        (Utilities|Time|ClearandInvalidateTimerbyHandle _firingtimer)))))

(event EventInteraction
  (params (Character :type BP%20Base%20Character%20Object%20Reference))
  ;[1 1 1] Interaction
  (CallFunction|Equip Character))

(fn ConstructionScript)