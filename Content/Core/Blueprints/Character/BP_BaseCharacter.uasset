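; Base character Blueprint providing movement states, weapon handling, health and death, with empty weapon and health info events.
; It spawns and equips StartWeapon, and aim, run and crouch events toggle state flags, speed, rotation mode and capsule height.
; Firing requires aiming; reloading refills the weapon on a montage notify, spending one Ammo map unit per magazine, with negative counts also allowed.
; Damage reduces HP until death drops the weapon and ragdolls the mesh.
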(event Custom|StartRunning
  ;[1 1 1] Run
  (if (not (Variables|Default|GetAiming))
    (if (Variables|Default|GetCrouching)
      (CallFunction|EventUncrouch)
      (else
        (Variables|Default|SetRunning true)))
    (Variables|/Script/Engine.CharacterMovementComponent|SetMaxWalkSpeed (Variables|Character|GetCharacterMovement) (Variables|Default|GetRunSpeed))))

(event Custom|StopRunning
  ;[1 1 1] Run
  (Variables|Default|SetRunning false)
  (Variables|/Script/Engine.CharacterMovementComponent|SetMaxWalkSpeed (Variables|Character|GetCharacterMovement) (Variables|Default|GetWalkSpeed)))

(event Custom|Death
  (bind _activeweapon (Variables|Default|GetActiveWeapon))
  (bind _capsulecomponent (Variables|Collision|GetCapsuleComponent))
  (bind _charactermovement (Variables|Character|GetCharacterMovement))
  (bind _mesh (Variables|Character|GetMesh))
  ;[1 1 1] Death
  (Variables|Default|SetDead true)
  (Utilities|IsValid _activeweapon
    (:Is%20Valid
      (Default|Drop _activeweapon))
    (:Is%20Not%20Valid
      _))
  (Components|Movement|StopMovementImmediately _charactermovement)
  (Pawn|Components|CharacterMovement|SetMovementMode _charactermovement "MOVE_None" 0)
  (Collision|SetCollisionResponsetoChannel _capsulecomponent "ECC_Pawn" "ECR_Ignore")
  (Collision|SetCollisionResponsetoChannel _capsulecomponent "ECC_Visibility" "ECR_Ignore")
  (Collision|SetCollisionResponsetoChannel _capsulecomponent "ECC_Camera" "ECR_Ignore")
  (Collision|SetCollisionEnabled _mesh "QueryAndPhysics")
  (Physics|SetSimulatePhysics _mesh true))

(event Custom|UpdateWeaponInfo
  ;[1 1 1] Reload
)

(event Custom|UpdateHealthInfo
  ;[1 1 1] Reload
)

(event Custom|EventUncrouch
  ;[1 1 1] Crouch
  (Variables|Default|SetCrouching false)
  (Variables|Default|SetRunning false)
  (Variables|/Script/Engine.CharacterMovementComponent|SetMaxWalkSpeed (Variables|Character|GetCharacterMovement) (Variables|Default|GetWalkSpeed))
  (Components|Capsule|SetCapsuleHalfHeight (Variables|Collision|GetCapsuleComponent) 88.0 true)
  (Transformation|SetRelativeLocation (Variables|Character|GetMesh) "0.000000,0.000000,-88.000000" false false))

(event Custom|EventCrouch
  ;[1 1 1] Crouch
  (Variables|Default|SetCrouching true)
  (if (Variables|Default|GetAiming)
    (CallFunction|StopAim))
  (Variables|/Script/Engine.CharacterMovementComponent|SetMaxWalkSpeed (Variables|Character|GetCharacterMovement) (Variables|Default|GetCrouchSpeed))
  (Components|Capsule|SetCapsuleHalfHeight (Variables|Collision|GetCapsuleComponent) 55.0 true)
  (Transformation|SetRelativeLocation (Variables|Character|GetMesh) "0.000000,0.000000,-54.000000" false false))

(event Custom|Aim
  ;[1 1 1] Aim
  (if (and (not (Variables|Default|GetRunning)) (Utilities|IsValid (Variables|Default|GetActiveWeapon)))
    (if (Variables|Default|GetCrouching)
      (CallFunction|EventUncrouch))
    (Variables|Default|SetAiming true)
    (Variables|/Script/Engine.CharacterMovementComponent|SetbOrientRotationToMovement (Variables|Character|GetCharacterMovement) false)))

(event Custom|Stop%20Aim
  (bind _activeweapon (Variables|Default|GetActiveWeapon))
  ;[1 1 1] Aim
  (Variables|Default|SetAiming false)
  (Variables|/Script/Engine.CharacterMovementComponent|SetbOrientRotationToMovement (Variables|Character|GetCharacterMovement) true)
  (Utilities|IsValid _activeweapon
    (:Is%20Valid
      (Default|StopFiring _activeweapon))))

(event Custom|StartFiring
  ;[1 1 1] Fire
  (if (Math|Boolean|ANDBoolean (Utilities|IsValid (Variables|Default|GetActiveWeapon)) (Variables|Default|GetAiming) (not (Variables|Default|GetReloading)))
    (Default|StartFiring (Variables|Default|GetActiveWeapon))))

(event Custom|StopFiring
  ;[1 1 1] Fire
  (if (and (Utilities|IsValid (Variables|Default|GetActiveWeapon)) (Variables|Default|GetAiming))
    (Default|StopFiring (Variables|Default|GetActiveWeapon))))

(event Custom|Reload
  (bind _activeweapon (Variables|Default|GetActiveWeapon))
  (bind _ammo (Variables|Default|GetAmmo))
  (bind _activeweapon_2 (Variables|Default|GetActiveWeapon))
  (bind _ammo_2 (Variables|Default|GetAmmo))
  (bind _activeweapon_3 (Variables|Default|GetActiveWeapon))
  (bind _ammotype (Variables|/Game/Core/Blueprints/Weapon/BP_WeaponBase.BP_WeaponBase_C|GetAmmoType _activeweapon))
  (bind _ammotype_2 (Variables|/Game/Core/Blueprints/Weapon/BP_WeaponBase.BP_WeaponBase_C|GetAmmoType _activeweapon_2))
  (bind (_value _returnvalue) (Utilities|Map|Find _ammo _ammotype_2))
  ;[1 1 1] Reload
  (if (not (Variables|Default|GetReloading))
    (Utilities|IsValid _activeweapon_2
      (:Is%20Valid
        (if _returnvalue
          (if (> _value 0)
            (Variables|Default|SetReloading true)
            (Animation|Montage|PlayMontage (Variables|Character|GetMesh) "/Game/AnimStarterPack/Reload_Rifle_Hip_Montage.Reload_Rifle_Hip_Montage" :!label _label
              (:OnNotifyBegin
                (Utilities|IsValid _activeweapon
                  (:Is%20Valid
                    (Variables|/Game/Core/Blueprints/Weapon/BP_WeaponBase.BP_WeaponBase_C|SetCurrentAmmo _activeweapon (Variables|/Game/Core/Blueprints/Weapon/BP_WeaponBase.BP_WeaponBase_C|GetMaxAmmo _activeweapon))
                    (bind _keys (Utilities|Map|Keys _ammo_2))
                    (bind _values (Utilities|Map|Values _ammo_2))
                    (Utilities|Map|Add _ammo_2 _ammotype (- (Utilities|Array|Get(acopy) _values (Utilities|Array|FindItem _keys _ammotype)) 1))
                    (Variables|Default|SetReloading false)
                    (CallFunction|UpdateWeaponInfo)
                    (Audio|PlaySoundatLocation (Variables|/Game/Core/Blueprints/Weapon/BP_WeaponBase.BP_WeaponBase_C|GetReloadSound _activeweapon_3) (Transformation|GetActorLocation _activeweapon_3) "0, 0, 0" 1.0 1.0 0.0 "/Game/MilitaryWeapDark/Sound/Attenuation/WeaponShot_att.WeaponShot_att" 0 0 0)))))
            (elif (< _value 0)
              (goto _label))))))))

(event Custom|StopReloading
  ;[1 1 1] Reload
  (if (Variables|Default|GetReloading)
    (Variables|Default|SetReloading false)
    (Animation|StopAnimMontage "/Game/AnimStarterPack/Reload_Rifle_Hip_Montage.Reload_Rifle_Hip_Montage")))

(event EventBeginPlay
  (bind _startweapon (Variables|Default|GetStartWeapon))
  (if (Utilities|IsValidClass _startweapon)
    (bind _returnvalue (Game|SpawnActorfromClass _startweapon (Math|Transform|MakeTransform "0, 0, 0" "0, 0, 0" "1.000000,1.000000,1.000000") "Undefined" "MultiplyWithRoot" 0 0))
    (Default|Equip _returnvalue self)))

(event Collision|EventActorBeginOverlap
  (params (OtherActor :type Actor%20Object%20Reference)))

(event EventTick
  (params (DeltaSeconds :type Float%20%28single-precision%29)))

(event Game|Damage|EventAnyDamage
  (params (Damage :type Float%20%28single-precision%29) (DamageType :type Damage%20Type%20Object%20Reference) (InstigatedBy :type Controller%20Object%20Reference) (DamageCauser :type Actor%20Object%20Reference))
  ;[1 1 1] Health System
  (if (not (Variables|Default|GetDead))
    (bind _output_get (Variables|Default|SetHP (- (Variables|Default|GetHP) Damage)))
    (if (<= _output_get 0.0)
      (CallFunction|Death))))

(fn ConstructionScript)