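; AI character Blueprint that handles aiming at a target, death, and being taken down by the player.
; While aiming, Tick turns it toward its target at a constant rate.
; A takedown area toggles CanTakedown on the overlapping player character, and Takedown disables movement and collision and plays an assassination montage.
; Death flags the blackboard; both endings fire OnDeath and destroy the actor, with delays.
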(event OnComponentBeginOverlap(TakedownArea)
  (params (OverlappedComponent :type Primitive%20Component%20Object%20Reference) (OtherActor :type Actor%20Object%20Reference) (OtherComp :type Primitive%20Component%20Object%20Reference) (OtherBodyIndex :type Integer) (bFromSweep :type Boolean) (SweepResult :type Hit%20Result%20Structure%20%28by%20ref%29))
  (bind _asbp_player_character (Utilities|Casting|CastToBP_PlayerCharacter OtherActor))
  (Variables|/Game/Core/Blueprints/Character/BP_PlayerCharacter.BP_PlayerCharacter_C|SetCanTakedown? _asbp_player_character true))

(event OnComponentEndOverlap(TakedownArea)
  (params (OverlappedComponent :type Primitive%20Component%20Object%20Reference) (OtherActor :type Actor%20Object%20Reference) (OtherComp :type Primitive%20Component%20Object%20Reference) (OtherBodyIndex :type Integer))
  (bind _asbp_player_character (Utilities|Casting|CastToBP_PlayerCharacter OtherActor))
  (Variables|/Game/Core/Blueprints/Character/BP_PlayerCharacter.BP_PlayerCharacter_C|SetCanTakedown? _asbp_player_character false))

(event Custom|Takedown
  (Pawn|Components|CharacterMovement|DisableMovement (Variables|Character|GetCharacterMovement))
  (Collision|SetActorEnableCollision false)
  (Animation|PlayAnimMontage "/Game/Core/Blueprints/Character/Animations/Takedown/AssassinationEnemy_Montage.AssassinationEnemy_Montage" 1.0 "None")
  (Utilities|FlowControl|Delay 1e+01)
  (Default|CallOnDeath)
  (Actor|DestroyActor))

(event EventBeginPlay
  (|CallParentFunction) ; This node is disabled and will not be called.\nDrag off pins to build functionality.
)

(event Collision|EventActorBeginOverlap
  (params (OtherActor :type Actor%20Object%20Reference))
  (|CallParentFunction OtherActor) ; This node is disabled and will not be called.\nDrag off pins to build functionality.
)

(event EventTick
  (params (DeltaSeconds :type Float%20%28single-precision%29))
  (bind _target (Variables|Default|GetTarget))
  (|CallParentFunction DeltaSeconds)
  (if (Variables|Default|GetAiming)
    (Utilities|IsValid _target
      (:Is%20Valid
        (Transformation|SetActorRotation (Class|KismetMathLibrary|RInterptoConstant (Transformation|GetActorRotation) (Math|Rotator|FindLookatRotation (Transformation|GetActorLocation) (Transformation|GetActorLocation _target)) DeltaSeconds 3.2e+02))))))

(event EventDeath
  (|CallParentFunction)
  (AI|Components|Blackboard|SetValueasBool (AI|GetBlackboard self) (Variables|Default|GetKey%20Name) true)
  (Default|CallOnDeath)
  (Utilities|FlowControl|Delay 3.0)
  (Actor|DestroyActor))

(fn ConstructionScript
  (|CallParentFunction))