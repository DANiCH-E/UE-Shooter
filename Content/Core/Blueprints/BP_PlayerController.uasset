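; BP_PlayerController is the player controller that opens and closes the game's pause state.
; The Pause input calls PauseEvent when not already paused, which pauses the game, switches to game-and-UI input with a visible cursor, and creates a WBP_PauseMenu widget.
; UnpauseEvent restores game-only input and hides the cursor, but does not remove the menu or get called within this Blueprint.
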(event Custom|UnpauseEvent
  (bind _returnvalue (Game|SetGamePaused false))
  (if _returnvalue
    (Variables|Default|SetIsPause false)
    (Input|SetInputModeGameOnly self false)
    (Variables|Default|SetbShowMouseCursor false)))

(event Custom|PauseEvent
  (bind _returnvalue (Game|SetGamePaused true))
  (if _returnvalue
    (Variables|Default|SetIsPause true)
    (Input|SetInputModeGameandUI self 0 "DoNotLock" true false)
    (Variables|Default|SetbShowMouseCursor true)
    (bind _returnvalue_2 (UserInterface|CreateWidget "/Game/Core/UI/WBP_PauseMenu.WBP_PauseMenu_C"))
    (UserInterface|Viewport|AddtoViewport _returnvalue_2 0)))

(event EventBeginPlay
  (Input|SetInputModeGameOnly self false))

(event Input|ActionEvents|InputActionPause
  (params (Key :type Key%20Structure :default "None"))
  (:Pressed
    (if (not (Variables|Default|GetIsPause))
      (CallFunction|PauseEvent))))

(fn ConstructionScript)