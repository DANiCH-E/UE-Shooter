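; Player character Blueprint that layers input, HUD, parkour and stealth takedowns over parent-class movement, weapon and health logic.
; A looping timer sphere-traces from the camera for interactables, while damage, health and weapon events refresh WBP_UI.
; Vaulting uses line traces for wall height and thickness to choose vault or get-up montages; takedowns align behind a traced AI for paired animation.
; Death shows a widget, then reloads ThirdPersonMap.
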(event EventBeginPlay
  (|CallParentFunction)
  (Utilities|FlowControl|Sequence
    (:then_0
      (Utilities|Time|SetTimerbyFunctionName 0 "InteractionCheck" 0.05 true))
    (:then_1
      (bind _returnvalue (UserInterface|CreateWidget "/Game/Core/UI/WBP_UI.WBP_UI_C"))
      (bind _output_get (Variables|Default|SetUIWidget _returnvalue))
      (UserInterface|Viewport|AddtoViewport _output_get 0)
      (Default|UpdateHealth (Variables|Default|GetUIWidget) (Variables|Default|GetHP) (Variables|Default|GetMaxHP))
      (Default|UpdateWeaponInfo (Variables|Default|GetUIWidget) (Variables|Default|GetActiveWeapon) self))))

(event Collision|EventActorBeginOverlap
  (params (OtherActor :type Actor%20Object%20Reference)))

(event EventDeath
  (|CallParentFunction)
  (Input|DisableInput self (Game|GetPlayerController 0))
  (Utilities|FlowControl|Delay 1.0)
  (bind _returnvalue (UserInterface|CreateWidget "/Game/Core/UI/WBP_Death.WBP_Death_C"))
  (UserInterface|Viewport|AddtoViewport _returnvalue 0)
  (Utilities|FlowControl|Delay 3.0)
  (Game|OpenLevel(byName) "ThirdPersonMap"))

(event EventTick
  (params (DeltaSeconds :type Float%20%28single-precision%29))
  ;[1 1 1] Aiming
  (Utilities|FlowControl|Sequence
    (:then_0
      (if (Variables|Default|GetAiming)
        (Transformation|SetActorRotation (Class|KismetMathLibrary|RInterptoConstant (Transformation|GetActorRotation) (Math|Rotator|MakeRotator 0.0 0.0 (.yaw (Pawn|GetControlRotation :!class /Script/Engine.Pawn))) DeltaSeconds 4.2e+02))))))

(event Game|Damage|EventAnyDamage
  (params (Damage :type Float%20%28single-precision%29) (DamageType :type Damage%20Type%20Object%20Reference) (InstigatedBy :type Controller%20Object%20Reference) (DamageCauser :type Actor%20Object%20Reference))
  (|CallParentFunction Damage DamageType InstigatedBy DamageCauser)
  (Default|UpdateHealth (Variables|Default|GetUIWidget) (Variables|Default|GetHP) (Variables|Default|GetMaxHP)))

(event EventUpdateWeaponInfo
  (bind _uiwidget (Variables|Default|GetUIWidget))
  (|CallParentFunction)
  (Utilities|IsValid _uiwidget
    (:Is%20Valid
      (Default|UpdateWeaponInfo _uiwidget (Variables|Default|GetActiveWeapon) self))))

(event EventUpdateHealthInfo
  (bind _uiwidget (Variables|Default|GetUIWidget))
  (|CallParentFunction)
  (Utilities|IsValid _uiwidget
    (:Is%20Valid
      (Default|UpdateHealth _uiwidget (Variables|Default|GetHP) (Variables|Default|GetMaxHP)))))

(event Input|ActionEvents|InputActionRun
  (params (Key :type Key%20Structure))
  ;[1 1 1] Run
  (:Pressed
    (CallFunction|StartRunning))
  (:Released
    (CallFunction|StopRunning)))

(event Input|ActionEvents|InputActionCrouch
  (params (Key :type Key%20Structure))
  ;[1 1 1] Crouch
  (:Pressed
    (if (Variables|Default|GetCrouching)
      (CallFunction|EventUncrouch)
      (else
        (CallFunction|EventCrouch)))))

(event Input|ActionEvents|InputActionInteraction
  (params (Key :type Key%20Structure))
  (bind _interactionactor (Variables|Default|GetInteractionActor))
  ;[1 1 1] Interaction
  (:Pressed
    (Utilities|IsValid _interactionactor
      (:Is%20Valid
        (Class|BIInteraction|Interaction(Message) _interactionactor self)))))

(event Input|ActionEvents|InputActionDrop
  (params (Key :type Key%20Structure))
  (bind _activeweapon (Variables|Default|GetActiveWeapon))
  ;[1 1 1] Drop Weapon
  (:Pressed
    (Utilities|IsValid _activeweapon
      (:Is%20Valid
        (if (Variables|Default|GetAiming)
          (CallFunction|StopAim))
        (CallFunction|StopReloading)
        (Default|Drop _activeweapon)))))

(event Input|ActionEvents|InputActionAim
  (params (Key :type Key%20Structure))
  (:Pressed
    (CallFunction|Aim))
  (:Released
    (CallFunction|StopAim)))

(event Input|ActionEvents|InputActionFire
  (params (Key :type Key%20Structure))
  (:Pressed
    (CallFunction|StartFiring))
  (:Released
    (CallFunction|StopFiring)))

(event Input|ActionEvents|InputActionReload
  (params (Key :type Key%20Structure))
  (:Pressed
    (CallFunction|Reload)))

(event Input|ActionEvents|InputActionVaulting
  (params (Key :type Key%20Structure))
  (bind _returnvalue (Transformation|GetActorLocation))
  (bind _returnvalue_2 (Transformation|GetActorRotation))
  (bind _returnvalue_3 (Transformation|GetActorLocation))
  (bind _returnvalue_4 (- _returnvalue "0.000000,0.000000,44.000000"))
  ;[1 1 1] Parkour
  (:Pressed
    (bind (_outhit _returnvalue_5) (Collision|LineTraceForObjects _returnvalue_4 (+ _returnvalue_4 (* (Transformation|GetActorForwardVector) 7e+01)) (Utilities|Array|MakeArray "ObjectTypeQuery1") true 0 "ForDuration"))
    (if _returnvalue_5
      (Variables|Default|SetWallLocation (.Location (Collision|BreakHitResult _outhit)))
      (Variables|Default|SetWallNormal (.Normal (Collision|BreakHitResult _outhit)))
      (bind (_outhit_2 _returnvalue_6) (Collision|LineTraceForObjects (+ (+ (Variables|Default|GetWallLocation) (* (Math|Vector|GetForwardVector (Math|Rotator|MakeRotfromX (Variables|Default|GetWallNormal))) -1e+01)) "0.000000,0.000000,200.000000") (- (+ (+ (Variables|Default|GetWallLocation) (* (Math|Vector|GetForwardVector (Math|Rotator|MakeRotfromX (Variables|Default|GetWallNormal))) -1e+01)) "0.000000,0.000000,200.000000") "0.000000,0.000000,200.000000") (Utilities|Array|MakeArray "ObjectTypeQuery1") true 0 "ForDuration"))
      (if _returnvalue_6
        (Variables|Default|SetWall%20Height (.Location (Collision|BreakHitResult _outhit_2)))
        (Utilities|FlowControl|Sequence
          (:then_0
            (if (> (.Z (Math|Vector|BreakVector (- (Variables|Default|GetWall%20Height) (Variables|Default|GetWallLocation)))) 6e+01)
              (Variables|Default|SetShouldClimb? true)
              (else
                (Variables|Default|SetShouldClimb? false))))
          (:then_1
            (bind (_outhit_3 _returnvalue_7) (Collision|LineTraceForObjects (+ (+ (Variables|Default|GetWallLocation) (* (Math|Vector|GetForwardVector (Math|Rotator|MakeRotfromX (Variables|Default|GetWallNormal))) -5e+01)) "0.000000,0.000000,250.000000") (- (+ (+ (Variables|Default|GetWallLocation) (* (Math|Vector|GetForwardVector (Math|Rotator|MakeRotfromX (Variables|Default|GetWallNormal))) -5e+01)) "0.000000,0.000000,250.000000") "0.000000,0.000000,300.000000") (Utilities|Array|MakeArray "ObjectTypeQuery1") true 0 "ForDuration"))
            (if _returnvalue_7
              (Variables|Default|SetWallHeight2 (.Location (Collision|BreakHitResult _outhit_3)))
              (Utilities|FlowControl|Sequence
                (:then_0
                  (if (> (.Z (Math|Vector|BreakVector (- (Variables|Default|GetWall%20Height) (Variables|Default|GetWallHeight2)))) 3e+01)
                    (Variables|Default|SetIsWallThick? false)
                    (else
                      (Variables|Default|SetIsWallThick? true))))
                (:then_1
                  (if (not (Variables|Default|GetShouldClimb?)) :!label _label
                    ;;[1 1 1] Vaulting And/Or getting up
                    (Collision|SetCollisionEnabled (Variables|Default|GetCapsuleComponent) "NoCollision")
                    (Pawn|Components|CharacterMovement|SetMovementMode (Variables|Character|GetCharacterMovement) "MOVE_Flying" 0)
                    (if (Variables|Default|GetIsWallThick?)
                      (Transformation|SetActorLocation (+ (Transformation|GetActorLocation) (* (Math|Vector|GetForwardVector (Math|Rotator|MakeRotfromX (Variables|Default|GetWallNormal))) 5e+01)) false false)
                      (bind _returnvalue_8 (Animation|PlayAnimMontage "/Game/Core/Blueprints/Character/Animations/MQ_GettingUp_RM_Montage.MQ_GettingUp_RM_Montage" 1.0 "None"))
                      (Utilities|FlowControl|Delay _returnvalue_8)
                      (else
                        (Transformation|SetActorLocation (+ (Transformation|GetActorLocation) (* (Math|Vector|GetForwardVector (Math|Rotator|MakeRotfromX (Variables|Default|GetWallNormal))) 5e+01)) false false)
                        (Transformation|SetActorLocation (Math|Vector|MakeVector (.x _returnvalue_3) (.y _returnvalue_3) (- (.Z (Math|Vector|BreakVector (Variables|Default|GetWall%20Height))) 2e+01)) false false)
                        (bind _returnvalue_9 (Animation|PlayAnimMontage "/Game/Core/Blueprints/Character/Animations/MQ_Vault_RM_Montage.MQ_Vault_RM_Montage" 1.0 "None"))
                        (Utilities|FlowControl|Delay _returnvalue_9)))
                    (Collision|SetCollisionEnabled (Variables|Default|GetCapsuleComponent) "QueryAndPhysics")
                    (Pawn|Components|CharacterMovement|SetMovementMode (Variables|Character|GetCharacterMovement) "MOVE_Walking" 0)
                    (Transformation|SetActorRotation (Math|Rotator|MakeRotator (.roll _returnvalue_2) (.pitch _returnvalue_2) (+ (.Yaw (Math|Rotator|BreakRotator (Math|Rotator|MakeRotfromX (Variables|Default|GetWallNormal)))) 1.8e+02))))))
              (else
                (Variables|Default|SetIsWallThick? false)
                (goto _label)))))))))

(event Input|ActionEvents|InputActionTakeDown
  (params (Key :type Key%20Structure))
  (bind _returnvalue (Transformation|GetActorLocation))
  ;[1 1 1] Stealth Kill
  (:Pressed
    (if (Variables|Default|GetCanTakedown?)
      (bind (_outhit _returnvalue_2) (Collision|LineTraceByChannel _returnvalue (+ _returnvalue (* (Transformation|GetActorForwardVector) 2.5e+02)) "TraceTypeQuery1" false 0 "None"))
      (if _returnvalue_2
        (bind _asbp_aicharacter (Utilities|Casting|CastToBP_AICharacter (.HitActor (Collision|BreakHitResult _outhit))))
        (Variables|Default|SetTakedownTarget _asbp_aicharacter)
        (Transformation|AttachComponentToComponent (Variables|Default|GetSpringArm) (Variables|Character|GetMesh) "spine_02" "SnapToTarget" "SnapToTarget" "SnapToTarget" true)
        (Pawn|Components|CharacterMovement|DisableMovement (Variables|Character|GetCharacterMovement))
        (Variables|Default|SetCanTakedown? false)
        (Transformation|SetActorTransform (Math|Transform|MakeTransform (+ (.location (Transformation|GetActorTransform (Variables|Default|GetTakedownTarget))) (* (Transformation|GetActorForwardVector (Variables|Default|GetTakedownTarget)) -175.0)) (.rotation (Transformation|GetActorTransform (Variables|Default|GetTakedownTarget))) "1.000000,1.000000,1.000000"))
        (bind _returnvalue_3 (Animation|PlayAnimMontage "/Game/Core/Blueprints/Character/Animations/Takedown/AssassinationAttacker_Montage.AssassinationAttacker_Montage" 1.0 "None"))
        (Default|Takedown (Variables|Default|GetTakedownTarget))
        (Utilities|FlowControl|Delay (+ _returnvalue_3 0.025))
        (Transformation|SetActorLocation (+ (Transformation|GetActorLocation) (* (Transformation|GetActorForwardVector) 175.0)) false false)
        (Pawn|Components|CharacterMovement|SetMovementMode (Variables|Character|GetCharacterMovement) "MOVE_Walking" 0)
        (Transformation|AttachComponentToComponent (Variables|Default|GetSpringArm) (Variables|Character|GetMesh) "spine_02" "KeepRelative" "KeepRelative" "KeepRelative" true)))))

(event Input|AxisEvents|InputAxisLookUp
  (params (AxisValue :type Float%20%28single-precision%29))
  ;[1 1 1] Camera
  (Pawn|Input|AddControllerPitchInput AxisValue))

(event Input|AxisEvents|InputAxisLookRight
  (params (AxisValue :type Float%20%28single-precision%29))
  ;[1 1 1] Camera
  (Pawn|Input|AddControllerYawInput AxisValue))

(event Input|AxisEvents|InputAxisMoveForward
  (params (AxisValue :type Float%20%28single-precision%29))
  ;[1 1 1] Movement
  (Pawn|Input|AddMovementInput (Math|Vector|GetForwardVector (Math|Rotator|MakeRotator 0.0 0.0 (.yaw (Pawn|GetControlRotation :!class /Script/Engine.Pawn)))) AxisValue false))

(event Input|AxisEvents|InputAxisMoveRight
  (params (AxisValue :type Float%20%28single-precision%29))
  (bind _returnvalue (Pawn|GetControlRotation :!class /Script/Engine.Pawn))
  ;[1 1 1] Movement
  (Pawn|Input|AddMovementInput (Math|Vector|GetRightVector (Math|Rotator|MakeRotator (.roll _returnvalue) 0.0 (.yaw _returnvalue))) AxisValue false))

(fn ConstructionScript
  (|CallParentFunction))

(fn InteractionCheck
  (bind _returnvalue (Game|GetPlayerCameraManager 0))
  (bind _uiwidget (Variables|Default|GetUIWidget))
  (bind _uiwidget_2 (Variables|Default|GetUIWidget))
  (bind _returnvalue_2 (Transformation|GetActorLocation _returnvalue))
  (bind (_outhit _returnvalue_3) (Collision|SphereTraceByChannel _returnvalue_2 (+ _returnvalue_2 (* (Transformation|GetActorForwardVector (Game|GetPlayerController 0)) 1e+03)) 3e+01 "TraceTypeQuery1" false 0 "None"))
  (if _returnvalue_3
    (if (Utilities|DoesObjectImplementInterface (.HitActor (Collision|BreakHitResult _outhit)) "/Game/Core/Blueprints/BI_Interaction.BI_Interaction_C")
      (Variables|Default|SetInteractionActor (.HitActor (Collision|BreakHitResult _outhit)))
      (Utilities|IsValid _uiwidget_2
        (:Is%20Valid
          (Variables|/Script/UMG.Widget|SetVisibility (Variables|/Game/Core/UI/WBP_UI.WBP_UI_C|GetInteractionText _uiwidget_2) "Visible")))
      (else
        (Variables|Default|SetInteractionActor 0 :!label _label)
        (Utilities|IsValid _uiwidget
          (:Is%20Valid
            (Variables|/Script/UMG.Widget|SetVisibility (Variables|/Game/Core/UI/WBP_UI.WBP_UI_C|GetInteractionText _uiwidget) "Hidden")))))
    (else
      (goto _label))))