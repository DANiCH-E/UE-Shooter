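; BP_NPC is an NPC blueprint that shows its dialogue one line per interaction.
; Each Interaction call increments a clamped TalkIndex, creates WB_Dialogue if needed, sets its text from the Dialogue array and plays a click sound.
; Past the last line it removes the widget.
; The index reset sits inside the in-range branch with a Length + 1 test, so it never fires and dialogue does not restart.
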(event EventInteraction
  (params (Character :type BP%20Base%20Character%20Object%20Reference))
  (bind _result (Math|Integer|IncrementInt (Variables|Default|GettalkIndex))
    (:%20%20
      (Variables|Default|SettalkIndex (Math|Integer|Clamp(Integer) _result 0 4))
      (if (< (Variables|Default|GettalkIndex) (Utilities|Array|Length (Variables|Default|GetDialogue)))
        (Variables|Default|GetUI
          (:then
            _)
          (:else
            (bind _returnvalue (UserInterface|CreateWidget "/Game/Core/UI/Dialogue/WB_Dialogue.WB_Dialogue_C" (Game|GetPlayerController 0)))
            (bind _output_get (Variables|Default|SetUI _returnvalue))
            (UserInterface|Viewport|AddtoViewport _output_get 0)))
        (Rendering|Components|TextRender|SetText (Variables|/Game/Core/UI/Dialogue/WB_Dialogue.WB_Dialogue_C|GetTalkText (Variables|Default|GetUI)) (Utilities|Text|ToText(String) (Utilities|Array|Get(acopy) (Variables|Default|GetDialogue) (Variables|Default|GettalkIndex))))
        (Audio|PlaySound2D "/Engine/VREditor/Sounds/UI/Click_on_Button.Click_on_Button" 1.0 1.0 0.0 0 0)
        (if (== (Variables|Default|GettalkIndex) (+ (Utilities|Array|Length (Variables|Default|GetDialogue)) 1))
          (Variables|Default|SettalkIndex -1))
        (else
          (Widget|RemovefromParent (Variables|Default|GetUI)))))))

(fn ConstructionScript)