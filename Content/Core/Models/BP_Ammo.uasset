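; BP_Ammo is an ammo pickup actor that adds rounds to a character's ammo map when interacted with.
; Its Interaction event looks up AmmoType in the character's Ammo map.
; An existing entry is increased by Amount, then the weapon info updates and the pickup is destroyed.
; A missing type is only inserted with Amount, without that update or destruction.
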(event EventBeginPlay)

(event Collision|EventActorBeginOverlap
  (params (OtherActor :type Actor%20Object%20Reference)))

(event EventTick
  (params (DeltaSeconds :type Float%20%28single-precision%29)))

(event EventInteraction
  (params (Character :type BP%20Base%20Character%20Object%20Reference))
  (bind _ammo (Variables|/Game/Core/Blueprints/Character/BP_BaseCharacter.BP_BaseCharacter_C|GetAmmo Character))
  (bind _ammotype (Variables|Default|GetAmmoType))
  (bind (_value _returnvalue) (Utilities|Map|Find _ammo _ammotype))
  (if _returnvalue
    (Utilities|Map|Add _ammo (Variables|Default|GetAmmoType) (+ _value (Variables|Default|GetAmount)))
    (Default|UpdateWeaponInfo Character)
    (Actor|DestroyActor)
    (else
      (Utilities|Map|Add _ammo (Variables|Default|GetAmmoType) (Variables|Default|GetAmount)))))

(fn ConstructionScript)